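; BP_Grid is a grate actor that opens and closes by sliding its static mesh by a configurable offset.
; On BeginPlay it stores the mesh's relative location as the start and adds OpeningHeight to get the final position.
; Togglegrate plays or reverses the GridAnimation timeline based on the Open flag, and its update lerps the mesh between the two positions.
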(event `self.ReceiveBeginPlay`
  (bind _output_get (set `self.StartPosition` (`SceneComponent.RelativeLocation` (`self.StaticMesh`))))
  (bind _output_get_2 (set `self.FinalPosition` (+ _output_get (`self.Opening Height`)))))

(event `Toggle grate`
  (params (Open :type Boolean))
  (if Open
    (bind (_direction _alpha) (`Timeline|GridAnimation` :!label _label)
      (:`Update`
        (`SceneComponent.K2_SetRelativeLocation` (`self.StaticMesh`) (`KismetMathLibrary.VLerp` (`self.StartPosition`) (stale `self.ReceiveBeginPlay` _output_get_2) _alpha) false false)))
    (else
      (goto _label :!via `Reverse`))))

(event `self.ReceiveActorBeginOverlap`
  (params (OtherActor :type "Actor Object Reference")))

(event `self.ReceiveTick`
  (params (DeltaSeconds :type "Float (single-precision)")))

(fn `UserConstructionScript`)