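; AC_Health is a health component that tracks current health and death state for its owning actor.
; On BeginPlay it fills health to the maximum and broadcasts the change event.
; TakeDamage subtracts damage clamped between zero and max, broadcasts and prints the new value, then sets IsDead and fires the death event once at zero, ignoring further damage.
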(event `self.ReceiveBeginPlay`
  (bind _output_get (set `self.CurrentHealth` (`self.MaxHealth`)))
  (`self.OnHealthChanged` _output_get (`self.MaxHealth`)))

(fn `TakeDamage`
  (params (DamageAmount :type "Float (double-precision)"))
  (if (not (`self.IsDead`))
    (bind _output_get (set `self.CurrentHealth` (`KismetMathLibrary.FClamp` (- (`self.CurrentHealth`) DamageAmount) 0.0 (`self.MaxHealth`))))
    (`self.OnHealthChanged` _output_get (`self.MaxHealth`))
    (`KismetSystemLibrary.PrintString` (`KismetStringLibrary.Conv_DoubleToString` (`self.CurrentHealth`)))
    (if (<= (`self.CurrentHealth`) 0.0)
      (set `self.IsDead` true)
      (`self.OnDeath`))))