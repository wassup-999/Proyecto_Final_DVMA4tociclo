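; BP_Lever is an interactable lever that toggles a linked grate.
; Each Interaction flips IsActive and plays or reverses the LeverAnimation timeline, which lerps the PivotHandle rotation between two opposite angles.
; When the timeline finishes in either direction, it passes the current state to GridObjetive's ToggleGrate if that reference is valid, so the grate reacts only after the handle completes its swing.
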(event `/Game/GamePlay/BPI_Interact.Interaction`
  (bind _gridobjetive (`self.GridObjetive`))
  (bind _output_get (set `self.IsActive` (not (`self.IsActive`))))
  (if _output_get
    (bind (_direction _alpha) (`Timeline|LeverAnimation` :!label _label)
      (:`Update`
        (`SceneComponent.K2_SetRelativeRotation` (`self.Pivot_handle`) (`KismetMathLibrary.RLerp` (struct :`Pitch` -35.0) (struct :`Pitch` 35.0) _alpha) false false))
      (:`Finished`
        (`/Engine/EditorBlueprintResources/StandardMacros.IsValid` _gridobjetive
          (:`Is Valid`
            (`/Game/GamePlay/BP_Grid.Toggle grate` _gridobjetive (`self.IsActive`))))))
    (else
      (goto _label :!via `Reverse`))))

(fn `UserConstructionScript`)